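; Projectile Blueprint for the Mage's staff light attack, the fourth variant by its name.
; On overlapping an ERNEnemyCharacter it disables its own collision, and the graph does nothing else live.
; Disconnected nodes hold an authority-only explosion damage calculation from owner attack power and weapon light attack damage, plus a call to hide the actor.
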(event `self.ReceiveBeginPlay`)

(event `self.ReceiveActorBeginOverlap`
  (params (OtherActor :type "Actor Object Reference"))
  (cast `ERNEnemyCharacter` OtherActor)
  (`self.SetActorEnableCollision` false))

(fn `UserConstructionScript`)