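; Mage staff Weapon Skill 4 projectile Blueprint, with almost no active logic of its own.
; On overlapping an ERNEnemyCharacter it disables its own collision; BeginPlay, Hit and the construction script are empty.
; Disconnected leftover nodes hold an authority-side damage and explosion damage calculation from the owner's attack power and equipped weapon, plus a debug print and a hide-actor call, none of which execute.
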(event `self.ReceiveBeginPlay`)

(event `self.ReceiveHit`
  (params (MyComp :type "PrimitiveComponent Object Reference") (Other :type "Actor Object Reference") (OtherComp :type "PrimitiveComponent Object Reference") (bSelfMoved :type Boolean) (HitLocation :type "Vector Structure") (HitNormal :type "Vector Structure") (NormalImpulse :type "Vector Structure") (Hit :type "HitResult Structure (by ref)"))
  ; Hit 판정 확인(Debug)
)

(event `self.ReceiveActorBeginOverlap`
  (params (OtherActor :type "Actor Object Reference"))
  (cast `ERNEnemyCharacter` OtherActor)
  (`self.SetActorEnableCollision` false))

(fn `UserConstructionScript`)