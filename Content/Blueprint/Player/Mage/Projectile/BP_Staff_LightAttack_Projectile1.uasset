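; Mage staff light-attack projectile that sets its own damage when spawned.
; On BeginPlay, only on the authority, it casts its owner to ProjectERNCharacter and sums AttackPower from the ERN attribute set with the equipped weapon's light-attack damage, scaled by a fixed multiplier.
; On any actor overlap it hides itself and disables collision, without destroying itself or applying damage in this graph.
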(event `self.ReceiveBeginPlay`
  (`/Engine/EditorBlueprintResources/ActorMacros.Switch Has Authority`
    (:`Authority`
      (bind _asproject_erncharacter (cast `ProjectERNCharacter` (`self.GetOwner`)))
      ; 캐릭터의 공격력
      (bind _returnvalue (`AbilitySystemComponent.GetAttributeSet` (`ERNCharacterBase.AbilitySystemComponent` _asproject_erncharacter) "/Script/ProjectERN.ERNAttributeSet"))
      (bind (_attackpower_basevalue _attackpower_currentvalue) (break `GameplayAttributeData` (`ERNAttributeSet.AttackPower` _returnvalue)))
      ; (캐릭터 공격력 + 무기 공격력) * 배수
      (set `self.Damage` (* (+ _attackpower_currentvalue (`ERNWeaponBase.LightAttackDamage` (`ERNEquipmentComponent.CurrentWeapon` (`self.GetComponentByClass` _asproject_erncharacter "/Script/ProjectERN.ERNEquipmentComponent")))) 0.8)))))

(event `self.ReceiveActorBeginOverlap`
  (params (OtherActor :type "Actor Object Reference"))
  (`self.SetActorHiddenInGame` true)
  (`self.SetActorEnableCollision` false))

(fn `UserConstructionScript`)