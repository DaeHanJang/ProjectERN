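; Director Blueprint for the lobby Level Sequence, providing event-track callbacks for an intro teleport cutscene.
; One event spawns the Niagara teleport effect at a stored location, then deactivates and destroys it after a six-second delay.
; Another clears players, destroying each ProjectERNCharacter and its weapon, but only where a current weapon is valid.
; Player_Walk is an empty stub, and a loop setting character walk velocity is left unconnected.
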(event `SequenceEvent`
  (bind _returnvalue (`NiagaraFunctionLibrary.SpawnSystemAtLocation` "/Game/Assets/VFX/CutScene/NS_Intro_Teleport.NS_Intro_Teleport" (`self.Location`)))
  (bind _output_get (set `self.Teleport` _returnvalue))
  (`KismetSystemLibrary.Delay` 6.0)
  (`ActorComponent.Deactivate` _output_get)
  (`ActorComponent.K2_DestroyComponent` _output_get))

(event `SequenceEvent_0`
  (bind _outactors (`GameplayStatics.GetAllActorsOfClass` "/Script/ProjectERN.ProjectERNCharacter"))
  (for _array_element _outactors
    (bind _currentweapon (`ERNEquipmentComponent.CurrentWeapon` (`ProjectERNCharacter.EquipmentComponent` _array_element)))
    ; 모든 플레이어 제거
    (`/Engine/EditorBlueprintResources/StandardMacros.IsValid` _currentweapon
      (:`Is Valid`
        (`Actor.K2_DestroyActor` _currentweapon)
        (`Actor.K2_DestroyActor` _array_element)))))

(event `Player_Walk`
  (params (Player1 :type "/Game/Blueprint/Player/Warrior/BP_Warrior1 Object Reference")))