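; BP_MoveBlock_R is a moving block actor whose RotationBlock component slides back and forth along its relative X axis.
; Each Tick, if the component is valid, it adds a game-time sine offset, scaled by MoveSpeed and MoveRanged, without sweeping.
; StartLocation is re-read from the current position every frame, so offsets accumulate and travel distance depends on frame rate.
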(event `self.ReceiveTick`
  (params (DeltaSeconds :type "Float (single-precision)"))
  (`/Engine/EditorBlueprintResources/StandardMacros.IsValid` (`self.RotationBlock`) :!label _label
    (:`Is Valid`
      (if true
        (bind _output_get (set `self.StartLocation` (`SceneComponent.RelativeLocation` (`self.RotationBlock`))))
        (`SceneComponent.K2_SetRelativeLocation` (`self.RotationBlock`) (+ _output_get (`KismetMathLibrary.MakeVector` (* (`KismetMathLibrary.Sin` (* (`KismetSystemLibrary.GetGameTimeInSeconds`) (`self.MoveSpeed`))) (`self.MoveRanged`)))) false false)
        (else
          (goto _label))))))

(fn `UserConstructionScript`)