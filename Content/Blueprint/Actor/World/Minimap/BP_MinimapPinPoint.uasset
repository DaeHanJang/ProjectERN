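; Minimap pin point actor that shows a cube colored according to which player pin it represents.
; On BeginPlay it creates a dynamic material instance on the cube and stores it as PinColor.
; ApplyPinColorbyIconType switches on the icon type and sets that material's Color parameter to red, blue or green for the three player pins.
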(event `self.ReceiveBeginPlay`
  (bind _returnvalue (`PrimitiveComponent.CreateDynamicMaterialInstance` (`self.Cube`) 0 null "Color"))
  (set `self.PinColor` _returnvalue))

(event `self.ApplyPinColorByIconType`
  (params (InIconType :type "EERNMinimapIconType Enum" :default "Building"))
  (switch `EERNMinimapIconType` InIconType
    (:`PlayerPin1`
      (`MaterialInstanceDynamic.SetVectorParameterValue` (`self.PinColor`) "Color" (struct :`R` 1.0 :`A` 1.0)))
    (:`PlayerPin2`
      (`MaterialInstanceDynamic.SetVectorParameterValue` (`self.PinColor`) "Color" (struct :`B` 255.0 :`A` 1.0)))
    (:`PlayerPin3`
      (`MaterialInstanceDynamic.SetVectorParameterValue` (`self.PinColor`) "Color" (struct :`G` 255.0 :`A` 1.0)))))

(fn `UserConstructionScript`)